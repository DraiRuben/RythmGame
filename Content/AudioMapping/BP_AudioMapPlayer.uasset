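; BP_AudioMapPlayer spawns notes for an audio-mapped game on upper and lower lanes.
; At BeginPlay it waits a tick, then caches the BP_NotePath from each lane's child actor.
; PlayNote uses note type to set whether the note hurts the player and lane to pick the path.
; Every type currently spawns BP_Note, passed the animation, path, arrival time and hurt flag.
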(event `self.ReceiveBeginPlay`
  (`KismetSystemLibrary.DelayUntilNextTick`)
  (set `self.UpperPath` (cast `/Game/AudioMapping/BP_NotePath` (`ChildActorComponent.ChildActor` (`self.BP_NotePathUpper`)) :!pure true))
  (set `self.LowerPath` (cast `/Game/AudioMapping/BP_NotePath` (`ChildActorComponent.ChildActor` (`self.BP_NotePathLower`)) :!pure true)))

(event `/Game/AudioMapping/Interfaces/BPI_NotePlayer.PlayNote`
  (params (NoteType :type "/Game/AudioMapping/Enums/ENoteType Enum" :default "NewEnumerator0") (NoteLane :type "/Game/AudioMapping/Enums/ENoteLane Enum" :default "NewEnumerator0") (NoteLength :type Integer) (SpawnTimeOffset :type "Float (double-precision)") (NoteAnim :type "PaperFlipbook Object Reference"))
  (`|ExecutionSequence`
    (:`then_0`
      (switch `/Game/AudioMapping/Enums/ENoteType` NoteType
        (:`NewEnumerator0`
          (set `self.NoteClassToSpawn` "/Game/AudioMapping/BP_Note.BP_Note_C")
          (set `self.HurtPlayer` false))
        (:`NewEnumerator1`
          (set `self.NoteClassToSpawn` "/Game/AudioMapping/BP_Note.BP_Note_C")
          (set `self.HurtPlayer` true))
        (:`NewEnumerator2`
          (set `self.NoteClassToSpawn` "/Game/AudioMapping/BP_Note.BP_Note_C")
          (set `self.HurtPlayer` true))))
    (:`then_1`
      (switch `/Game/AudioMapping/Enums/ENoteLane` NoteLane
        (:`NewEnumerator0`
          (set `self.NoteLaneToSpawn` (`self.LowerPath`)))
        (:`NewEnumerator1`
          (set `self.NoteLaneToSpawn` (`self.UpperPath`)))))
    (:`then_2`
      (`|SpawnActorFromClass` (`self.NoteClassToSpawn`) (`KismetMathLibrary.MakeTransform` (1000.0 1000.0 1000.0)) "Undefined" "MultiplyWithRoot" null NoteAnim (`self.NoteLaneToSpawn`) SpawnTimeOffset (`self.HurtPlayer`) null))))

(fn `UserConstructionScript`)