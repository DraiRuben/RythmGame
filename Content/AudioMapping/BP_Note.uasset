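; Rhythm-game note that travels along a spline to the hit circle, then an exit spline at matched speed before despawning.
; SmashNote stops movement, awards fever, combo and fixed-precision score, and disables pawn collision; only zero-length notes then play a destroy trajectory.
; Long notes build a scaled flipbook trail and end marker at BeginPlay from note length and receiver distance.
; Notes flagged HurtPlayer damage the player on overlap.
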(event `self.ReceiveBeginPlay`
  ;[1 0.9141 0] Init
  (`PaperFlipbookComponent.SetFlipbook` (`self.Sprite`) (`self.NoteAnim`))
  (set `self.PathLength` (`SplineComponent.GetSplineLength` (`/Game/AudioMapping/BP_NotePath.PathSpline` (`self.Path`))))
  (set `self.ExitLength` (`SplineComponent.GetSplineLength` (`/Game/AudioMapping/BP_NotePath.ExitSpline` (`self.Path`))))
  (`self.TryConstructLongNote`)
  (`self.Move`))

(event `Move`
  ;[0.5937 1 0] Move To Hit Circle
  (`TimelineComponent.SetPlayRate` (`self.MoveRoutine`) (/ 1.0 (`self.TimeToArrive`)))
  (bind (_direction _routine) (`Timeline|MoveRoutine` :!label _label)
    (:`Update`
      (`self.K2_SetActorLocation` (`SplineComponent.GetLocationAtDistanceAlongSpline` (`/Game/AudioMapping/BP_NotePath.PathSpline` (`self.Path`)) (`KismetMathLibrary.Lerp` 0.0 (`self.PathLength`) _routine) "World")))
    (:`Finished`
      ;[0.125 0 1] Move After Hit Circle
      (`TimelineComponent.SetPlayRate` (`self.ExitRoutine`) (/ 1.0 (/ (* (`self.ExitLength`) (`self.TimeToArrive`)) (`self.PathLength`))))
      (bind (_direction_2 _routine_2) (`Timeline|ExitRoutine` :!label _label_2)
        (:`Update`
          (`self.K2_SetActorLocation` (`SplineComponent.GetLocationAtDistanceAlongSpline` (`/Game/AudioMapping/BP_NotePath.ExitSpline` (`self.Path`)) (`KismetMathLibrary.Lerp` 0.0 (`self.ExitLength`) _routine_2) "World")))
        (:`Finished`
          (`KismetSystemLibrary.Delay` 3.0)
          (`self.K2_DestroyActor`))))))

(event `SmashNote`
  (bind _returnvalue (`GameplayStatics.GetGameState`))
  ;[0 0.8125 1] Note smash
  (`|ExecutionSequence`
    (:`then_0`
      (goto _label :!via `Stop`))
    (:`then_1`
      (goto _label_2 :!via `Stop`))
    (:`then_2`
      (message `/Game/Systems/BPI_Gamestate.AddFever` _returnvalue 5)
      (message `/Game/Systems/BPI_Gamestate.IncreaseCombo` _returnvalue 1)
      (message `/Game/Systems/BPI_Gamestate.AddScore` _returnvalue 10 "NewEnumerator0"))
    (:`then_3`
      (`self.SmashNoteFeedback`))
    (:`then_4`
      (`PrimitiveComponent.SetCollisionResponseToChannel` (`self.CapsuleComponent`) "ECC_Pawn" "ECR_Ignore")
      (set `self.Indestructible` true)
      (if (== (`self.NoteLength`) 0.0)
        (`TimelineComponent.SetPlayRate` (`self.DestroyTrajectory`) (/ 1.0 (`self.TimeToDie`)))
        (bind (_direction _trajectory) (`Timeline|DestroyTrajectory` :!via `PlayFromStart`)
          (:`Update`
            (`self.K2_AddActorWorldOffset` _trajectory))
          (:`Finished`
            (`self.K2_DestroyActor`)))))))

(event `self.CapsuleComponent.OnComponentBeginOverlap`
  (params (OverlappedComponent :type "PrimitiveComponent Object Reference") (OtherActor :type "Actor Object Reference") (OtherComp :type "PrimitiveComponent Object Reference") (OtherBodyIndex :type Integer) (bFromSweep :type Boolean) (SweepResult :type "HitResult Structure (by ref)"))
  ;[0 1 0.7891] Player overlap
  (if (`self.HurtPlayer`)
    (bind _asbp_player (cast `/Game/Player/BP_Player` OtherActor))
    (`KismetSystemLibrary.PrintString` "off")
    (`/Game/Player/BP_Player.Hurt` _asbp_player 15)
    (`PrimitiveComponent.SetCollisionResponseToChannel` (`self.CapsuleComponent`) "ECC_Pawn" "ECR_Ignore")))

(fn `GetCurrentPrecision`
  (returns (Precision :type "/Game/AudioMapping/Enums/ENotePrecision Enum"))
  (return "NewEnumerator0"))

(fn `SmashNoteFeedback`)

(fn `TryConstructLongNote`
  (locals (DistNoteToReceiver :type "Float (double-precision)"))
  (bind (_returnvalue_inputkey _returnvalue_position) (break `SplinePoint` (`SplineComponent.GetSplinePointAt` (`/Game/AudioMapping/BP_NotePath.PathSpline` (`self.Path`)) 1 "World")))
  (if (> (`self.NoteLength`) 0.0)
    (`|ExecutionSequence`
      (:`then_0`
        ;[0.8984 0 1] Get distance to receiver
        (set `local.DistNoteToReceiver` (`KismetMathLibrary.Vector_Distance` _returnvalue_position (`SceneComponent.K2_GetComponentLocation` (`self.Sprite`)))))
      (:`then_1`
        ;[0 0.5781 1] Instantiate long note path
        (bind _returnvalue (`AddComponent|NODE_AddPaperFlipbookComponent-0` :`bManualAttachment` true))
        (`SceneComponent.K2_AttachToComponent` _returnvalue (`self.CapsuleComponent`) "None" "KeepWorld" "KeepWorld" "KeepWorld" false)
        (`PaperFlipbookComponent.SetFlipbook` _returnvalue "/Game/Assets/Graphic/Beats/Long1/Flip_LongNotePath.Flip_LongNotePath")
        (`PrimitiveComponent.SetMaterial` _returnvalue 0 "/Game/Assets/Graphic/Beats/Long1/T_RepeatPath_Inst.T_RepeatPath_Inst")
        (`PrimitiveComponent.SetTranslucencySortDistanceOffset` _returnvalue 1.0)
        (`SceneComponent.SetWorldScale3D` _returnvalue (`KismetMathLibrary.MakeVector` (* (/ (`local.DistNoteToReceiver`) (.x (`.BoxExtent` (`KismetSystemLibrary.GetComponentBounds` _returnvalue)))) (/ (`self.NoteLength`) 2.0)) 1.0 3.65))
        (bind (_origin _boxextent) (`KismetSystemLibrary.GetComponentBounds` _returnvalue))
        (`SceneComponent.K2_SetWorldLocation` _returnvalue (+ (`SceneComponent.K2_GetComponentLocation` (`self.Sprite`)) (`KismetMathLibrary.MakeVector` (.x _boxextent) 0.0 (* (.z _boxextent) -1.0))) false false))
      (:`then_2`
        ;[0.07812 0 1] Instantiate exit note
        (bind _returnvalue_2 (`AddComponent|NODE_AddPaperFlipbookComponent-1` :`bManualAttachment` true))
        (`SceneComponent.K2_AttachToComponent` _returnvalue_2 (`self.CapsuleComponent`) "None" "SnapToTarget" "KeepWorld" "KeepWorld" false)
        (`PaperFlipbookComponent.SetFlipbook` _returnvalue_2 "/Game/Assets/Graphic/Beats/Long1/Flip_LongNote.Flip_LongNote")
        (`SceneComponent.K2_SetWorldLocation` _returnvalue_2 (+ (* (`SceneComponent.GetForwardVector` (`self.Sprite`)) (* (/ (* (`local.DistNoteToReceiver`) (`self.NoteLength`)) (`self.TimeToArrive`)) 2.0)) (`SceneComponent.K2_GetComponentLocation` (`self.Sprite`))) false false)))))

(fn `UserConstructionScript`)