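; BP_NoteReceiver is a hit zone that tracks BP_Note actors overlapping it so they can be smashed.
; Begin and end overlap events add and remove notes from the InRangeNotes array, with no duplicates.
; TryAttackNote calls SmashNote on the first note in the array, the earliest still in range, then removes it, and does nothing when the array is empty.
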(event `self.ReceiveActorBeginOverlap`
  (params (OtherActor :type "Actor Object Reference"))
  (bind _asbp_note (cast `/Game/AudioMapping/BP_Note` OtherActor))
  (`KismetArrayLibrary.Array_AddUnique` (`self.InRangeNotes`) _asbp_note))

(event `self.ReceiveActorEndOverlap`
  (params (OtherActor :type "Actor Object Reference"))
  (bind _asbp_note (cast `/Game/AudioMapping/BP_Note` OtherActor))
  (`KismetArrayLibrary.Array_RemoveItem` (`self.InRangeNotes`) _asbp_note))

(event `/Game/AudioMapping/BPI_NoteReceiver.TryAttackNote`
  (bind _inrangenotes (`self.InRangeNotes`))
  (bind _output (`|GetArrayItem` _inrangenotes))
  (if (> (`KismetArrayLibrary.Array_Length` _inrangenotes) 0)
    (`/Game/AudioMapping/BP_Note.SmashNote` _output)
    (`KismetArrayLibrary.Array_RemoveItem` _inrangenotes _output)))

(fn `UserConstructionScript`)