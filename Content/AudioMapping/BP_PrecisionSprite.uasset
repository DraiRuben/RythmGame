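; BP_PrecisionSprite is a short-lived floating sprite actor that displays a configurable sprite, likely as precision feedback in the audio-mapping game.
; On BeginPlay it applies a small random pitch, lifts itself and sets its sprite.
; A movement timeline then offsets it over its Lifetime while, after FullOpacityTime, an opacity timeline fades it and destroys the actor on finish.
; Both timelines scale their play rates to fit these durations.
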(event `self.ReceiveBeginPlay`
  (`self.K2_AddActorWorldRotation` (`KismetMathLibrary.MakeRotator` 0.0 (`KismetMathLibrary.RandomFloatInRange` -10.0 10.0)))
  (`self.K2_AddActorWorldOffset` (0.0 0.0 300.0))
  (`PaperSpriteComponent.SetSprite` (`self.RenderComponent`) (`self.Sprite`))
  (`|ExecutionSequence`
    (:`then_0`
      (`TimelineComponent.SetPlayRate` (`self.MovementTimeline`) (/ 1.0 (`self.Lifetime`)))
      (bind (_direction _offset) (`Timeline|MovementTimeline`)
        (:`Update`
          (`self.K2_AddActorWorldOffset` _offset))))
    (:`then_1`
      (`KismetSystemLibrary.Delay` (`self.FullOpacityTime`))
      (`TimelineComponent.SetPlayRate` (`self.OpacityTimeline`) (/ 1.0 (- (`self.Lifetime`) (`self.FullOpacityTime`))))
      (bind (_direction_2 _alpha) (`Timeline|OpacityTimeline`)
        (:`Update`
          (`PaperSpriteComponent.SetSpriteColor` (`self.RenderComponent`) (make `LinearColor` 1.0 1.0 1.0 _alpha)))
        (:`Finished`
          (`self.K2_DestroyActor`))))))

(fn `UserConstructionScript`)