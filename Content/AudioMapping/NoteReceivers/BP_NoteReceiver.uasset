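; BP_NoteReceiver is a lane hit zone for a rhythm game that turns attacks into note hits and player lane changes.
; Collider overlaps track notes in range, and scanning discards indestructible ones before taking the first remaining note.
; An attack smashes that note and forces the lane change, while misses request an unforced one, depending on void-attack permission and current lane.
; Long notes are returned for holding and releasing through indexed slots.
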(event `self.ReceiveBeginPlay`
  (`KismetSystemLibrary.DelayUntilNextTick`)
  (bind _player (message `/Game/Systems/BPI_Gamestate.GetPlayer` (`GameplayStatics.GetGameState`)))
  (set `self.Player` _player))

(event `self.Collider.OnComponentBeginOverlap`
  (params (OverlappedComponent :type "PrimitiveComponent Object Reference") (OtherActor :type "Actor Object Reference") (OtherComp :type "PrimitiveComponent Object Reference") (OtherBodyIndex :type Integer) (bFromSweep :type Boolean) (SweepResult :type "HitResult Structure (by ref)"))
  (bind _asbp_note (cast `/Game/AudioMapping/BP_Note` OtherActor))
  (`KismetArrayLibrary.Array_AddUnique` (`self.InRangeNotes`) _asbp_note))

(event `self.Collider.OnComponentEndOverlap`
  (params (OverlappedComponent :type "PrimitiveComponent Object Reference") (OtherActor :type "Actor Object Reference") (OtherComp :type "PrimitiveComponent Object Reference") (OtherBodyIndex :type Integer))
  (bind _asbp_note (cast `/Game/AudioMapping/BP_Note` OtherActor))
  (`KismetArrayLibrary.Array_RemoveItem` (`self.InRangeNotes`) _asbp_note))

(fn `ScanForNote`
  (returns (`LongNote?` :type Boolean) (NoteHandle :type "/Game/AudioMapping/BP_Note Object Reference"))
  (locals (Note :type "/Game/AudioMapping/BP_Note Object Reference") (ElementsToRemove :type "Array of /Game/AudioMapping/BP_Note Object Reference"))
  (bind _note (`local.Note`))
  ;[0 1 0.08594] Checks for any notes that would have become indestructible (by dealing damage to the player) and remove them from the array before trying to hit anything
  (if (`self.AreThereNotesInRange`)
    (for _array_element (`self.InRangeNotes`)
      (if (`/Game/AudioMapping/BP_Note.Indestructible` _array_element)
        (`KismetArrayLibrary.Array_Add` (`local.ElementsToRemove`) _array_element)))
    (for _array_element_2 (`local.ElementsToRemove`)
      (`KismetArrayLibrary.Array_RemoveItem` (`self.InRangeNotes`) _array_element_2))
    (if (`self.AreThereNotesInRange`)
      (set `local.Note` (`|GetArrayItem` (`self.InRangeNotes`)))
      (`KismetArrayLibrary.Array_RemoveItem` (`self.InRangeNotes`) (`local.Note`))
      (if (> (`/Game/AudioMapping/BP_Note.NoteLength` (`local.Note`)) 0.0)
        (return true _note)
        (else
          (return false _note)))
      (else
        (return false null)))
    (else
      (return false null))))

(fn `TryAttackLane`
  (params (AllowVoidAttacks :type Boolean))
  (returns (LongNoteHandle :type "/Game/AudioMapping/BP_Note Object Reference"))
  (locals (FoundNote :type "/Game/AudioMapping/BP_Note Object Reference"))
  (bind (_longnote_ _notehandle) (`self.ScanForNote`))
  (bind _output_get (set `local.FoundNote` _notehandle))
  (`/Engine/EditorBlueprintResources/StandardMacros.IsValid` _output_get
    (:`Is Valid`
      (`/Game/AudioMapping/BP_Note.SmashNote` _output_get self)
      (`/Game/Player/BP_Player.TryChangeLane` (`self.Player`) (`self.LanePos`) true)
      (if _longnote_ :!label _label
        _
        (else
          (return null))))
    (:`Is Not Valid`
      (if AllowVoidAttacks
        _
        (elif (`|EnumEquality` (`/Game/Player/BP_Player.CurrentLanePosition` (`self.Player`)) (`self.LanePos`))
          (return null)
          (else
            _)))
      (`/Game/Player/BP_Player.TryChangeLane` (`self.Player`) (`self.LanePos`) false)
      (goto _label)))
  (return (`local.FoundNote`)))

(fn `TryHoldNote`
  (params (NoteHandle :type "/Game/AudioMapping/BP_Note Object Reference") (Index :type Integer))
  (`KismetArrayLibrary.Array_Set` (`self.HeldNotes`) Index NoteHandle)
  (`/Engine/EditorBlueprintResources/StandardMacros.IsValid` NoteHandle
    (:`Is Valid`
      (`/Game/AudioMapping/BP_Note.StartHoldingNote` NoteHandle self)
      (`KismetArrayLibrary.Array_RemoveItem` (`self.InRangeNotes`) NoteHandle))))

(fn `TryStopHoldingNote`
  (params (Index :type Integer))
  (bind _heldnotes (`self.HeldNotes`))
  (bind _output (`|GetArrayItem` _heldnotes Index))
  (`/Engine/EditorBlueprintResources/StandardMacros.IsValid` _output
    (:`Is Valid`
      (`/Game/AudioMapping/BP_Note.StopHoldingNote` _output)
      (`KismetArrayLibrary.Array_Set` _heldnotes Index))))

(fn `UserConstructionScript`)