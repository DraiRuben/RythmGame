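; BP_NoteReceiver_Lower is a child note receiver that handles the lower-lane inputs for hitting notes.
; Three lower-lane input actions share identical logic on Started.
; Each asks the Player to try a lane change when its CurrentLanePosition equals one specific enum value, then calls TryAttackNote.
; BeginPlay and construction only call the parent, which suggests the core receiver logic is inherited.
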(event `self.ReceiveBeginPlay`
  (`parent.ReceiveBeginPlay`))

(event `EnhancedInput|/Game/Input/LowerLane/IA_LowerLane1`
  (params (ActionValue :type Boolean) (ElapsedSeconds :type "Float (double-precision)") (TriggeredSeconds :type "Float (double-precision)") (InputAction :type "InputAction Object Reference" :default "/Game/Input/LowerLane/IA_LowerLane1.IA_LowerLane1"))
  (bind _player (`self.Player`))
  (:`Started`
    (`|ExecutionSequence`
      (:`then_0`
        (if (`|EnumEquality` (`/Game/Player/BP_Player.CurrentLanePosition` _player) "NewEnumerator1")
          (`/Game/Player/BP_Player.TryChangeLane` _player)))
      (:`then_1`
        (`self.TryAttackNote`)))))

(event `EnhancedInput|/Game/Input/LowerLane/IA_LowerLane2`
  (params (ActionValue :type Boolean) (ElapsedSeconds :type "Float (double-precision)") (TriggeredSeconds :type "Float (double-precision)") (InputAction :type "InputAction Object Reference" :default "/Game/Input/LowerLane/IA_LowerLane2.IA_LowerLane2"))
  (bind _player (`self.Player`))
  (:`Started`
    (`|ExecutionSequence`
      (:`then_0`
        (if (`|EnumEquality` (`/Game/Player/BP_Player.CurrentLanePosition` _player) "NewEnumerator1")
          (`/Game/Player/BP_Player.TryChangeLane` _player)))
      (:`then_1`
        (`self.TryAttackNote`)))))

(event `EnhancedInput|/Game/Input/LowerLane/IA_LowerLane0`
  (params (ActionValue :type Boolean) (ElapsedSeconds :type "Float (double-precision)") (TriggeredSeconds :type "Float (double-precision)") (InputAction :type "InputAction Object Reference" :default "/Game/Input/LowerLane/IA_LowerLane0.IA_LowerLane0"))
  (bind _player (`self.Player`))
  (:`Started`
    (`|ExecutionSequence`
      (:`then_0`
        (if (`|EnumEquality` (`/Game/Player/BP_Player.CurrentLanePosition` _player) "NewEnumerator1")
          (`/Game/Player/BP_Player.TryChangeLane` _player)))
      (:`then_1`
        (`self.TryAttackNote`)))))

(fn `UserConstructionScript`
  (`parent.UserConstructionScript`))