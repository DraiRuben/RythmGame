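; Upper-lane note receiver for a rhythm game, registering itself on the Player one tick after BeginPlay.
; IA_UpperLane input resolves the changed key index to attack the lane and start or stop long-note holds.
; Its buffer logic pairs double notes: a note waits if the lower receiver has one at nearly equal distance.
; If the lower receiver already buffered one, both smash with one sound and the player is forced to change lane.
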(event `self.ReceiveBeginPlay`
  (`parent.ReceiveBeginPlay`)
  (`KismetSystemLibrary.DelayUntilNextTick`)
  (set `/Game/Player/BP_Player.UpperReceiver` self (`self.Player`)))

(event `EnhancedInput|/Game/Input/IA_UpperLane`
  (params (ActionValue :type "Vector Structure") (ElapsedSeconds :type "Float (double-precision)") (TriggeredSeconds :type "Float (double-precision)") (InputAction :type "InputAction Object Reference" :default "/Game/Input/IA_UpperLane.IA_UpperLane"))
  (:`Triggered`
    (bind _index (`self.GetIndexThatChanged` ActionValue :!label _label))
    (if (!= _index -1)
      (bind (_longnotehandle _hasputnoteinbuffer) (`self.TryAttackLane` false _index))
      (if (not _hasputnoteinbuffer)
        (`self.TryHoldNote` _longnotehandle _index))))
  (:`Started`
    (goto _label))
  (:`Canceled`
    (bind _index_2 (`self.GetIndexThatChanged` ActionValue :!label _label_2))
    (if (!= _index_2 -1)
      (`self.TryStopHoldingNote` _index_2)))
  (:`Completed`
    (goto _label_2)))

(fn `TryToPutNoteInBuffer`
  (params (Note :type "/Game/AudioMapping/BP_Note Object Reference") (InputIndex :type Integer))
  (returns (HasPutNoteInBuffer :type Boolean) (HasTriggeredDouble :type Boolean))
  (locals (NoteToTreat :type "/Game/AudioMapping/BP_Note Object Reference") (OtherNoteInBuffer :type "/Game/AudioMapping/BP_Note Object Reference") (OtherReceiver :type "/Game/AudioMapping/NoteReceivers/BP_NoteReceiver Object Reference"))
  (bind _lowerreceiver (`/Game/Player/BP_Player.LowerReceiver` (`self.Player`)))
  (bind _inrangenotes (`/Game/AudioMapping/NoteReceivers/BP_NoteReceiver.InRangeNotes` _lowerreceiver))
  (set `local.NoteToTreat` Note)
  (set `local.OtherNoteInBuffer` (`/Game/AudioMapping/NoteReceivers/BP_NoteReceiver.NoteInBuffer` _lowerreceiver))
  (set `local.OtherReceiver` _lowerreceiver)
  (`/Engine/EditorBlueprintResources/StandardMacros.IsValid` (`local.OtherNoteInBuffer`)
    (:`Is Valid`
      (`/Game/AudioMapping/BP_Note.SmashNote` (`local.OtherNoteInBuffer`) (`local.OtherReceiver`) false)
      (`/Game/AudioMapping/BP_Note.SmashNote` (`local.NoteToTreat`) self true)
      (`|ExecutionSequence`
        (:`then_0`
          (if (> (`/Game/AudioMapping/BP_Note.NoteLength` (`local.NoteToTreat`)) 0.0)
            (`self.TryHoldNote` (`local.NoteToTreat`) InputIndex)))
        (:`then_1`
          (if (> (`/Game/AudioMapping/BP_Note.NoteLength` (`local.OtherNoteInBuffer`)) 0.0)
            (`self.TryHoldNote` (`local.OtherReceiver`) (`local.OtherNoteInBuffer`) (`/Game/AudioMapping/NoteReceivers/BP_NoteReceiver.InputIndexBuffer` (`local.OtherReceiver`)))))
        (:`then_2`
          (`/Game/Player/BP_Player.TryChangeLane` (`self.Player`) "NewEnumerator2" true)
          (`self.ResetNoteBuffer` (`local.OtherReceiver`))
          (return false true))))
    (:`Is Not Valid`
      (if (> (`KismetArrayLibrary.Array_Length` _inrangenotes) 0)
        (if (< (`KismetMathLibrary.Abs` (- (`/Game/AudioMapping/BP_Note.GetDistanceToReceiver` (`|GetArrayItem` _inrangenotes)) (`/Game/AudioMapping/BP_Note.GetDistanceToReceiver` (`local.NoteToTreat`)))) 10.0)
          (set `self.InputIndexBuffer` InputIndex)
          (`self.EnableNoteBuffer` (`local.NoteToTreat`))
          (return true false)
          (else
            _)))
      (return false false))))

(fn `UserConstructionScript`
  (`parent.UserConstructionScript`))