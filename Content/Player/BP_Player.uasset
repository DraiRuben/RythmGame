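; Player for a two-lane rhythm game that switches between upper and lower lanes, plays attack animations and takes damage from notes.
; Timelines lerp its height for lane changes and a manual gravity fall from the upper lane, held off while notes are held.
; Unforced inputs during transitions go into a short Tick-driven buffer.
; Lane changes and hits grant temporary invincibility via capsule collision, and hits send life changes to the GameState.
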(event `self.ReceiveBeginPlay`
  ;[0.1484 0 1] Init
  (set `/Game/Systems/BP_GameState.Player` self (cast `/Game/Systems/BP_GameState` (`GameplayStatics.GetGameState`) :!pure true)))

(event `Invincibility`
  (params (Duration :type "Float (double-precision)"))
  (bind _capsulecomponent (`self.CapsuleComponent`))
  ;[1 0 0.5625] Invincibility
  (`/Engine/EditorBlueprintResources/StandardMacros.DoOnce` false :!label _label
    (:`Completed`
      (`PrimitiveComponent.SetCollisionResponseToAllChannels` _capsulecomponent "ECR_Ignore")
      (`KismetSystemLibrary.Delay` Duration)
      (`PrimitiveComponent.SetCollisionResponseToAllChannels` _capsulecomponent "ECR_Overlap")
      (goto _label :!via `Reset`))))

(event `GoToUpperLane`
  (bind (_returnvalue_x _returnvalue_y) (`KismetMathLibrary.BreakVector` (`self.K2_GetActorLocation`)))
  (bind (_returnvalue_x_2 _returnvalue_y_2 _returnvalue_z) (`KismetMathLibrary.BreakVector` (`self.K2_GetActorLocation`)))
  (bind _lowerlanez (`self.LowerLaneZ`))
  ;[1 0 0.375] Upper Lane Change
  (`|ExecutionSequence`
    (:`then_0`
      (`TimelineComponent.SetPlayRate` (`self.JumpRoutine`) (/ 1.0 (`self.LaneChangeTime`)))
      (`|ExecutionSequence`
        (:`then_0`
          (`self.StopAutoFall`))
        (:`then_1`
          (bind (_direction _alpha) (`Timeline|JumpRoutine` :`NewTime` (/ (- _returnvalue_z _lowerlanez) (- (`self.UpperLaneZ`) _lowerlanez)) :!via `SetNewTime` :!label _label_2)
            (:`Update`
              (`self.K2_SetActorLocation` (`KismetMathLibrary.MakeVector` _returnvalue_x _returnvalue_y (`KismetMathLibrary.Lerp` (`self.LowerLaneZ`) (`self.UpperLaneZ`) _alpha))))
            (:`Finished`
              (set `self.IsInTransitionAnimation` false)
              (if (<= (`self.NoteHeldCount`) 0)
                (`self.GravityFalls`)))))
        (:`then_2`
          (goto _label_2))))
    (:`then_1`
      (`self.Invincibility` 0.3))
    (:`then_2`
      (if (and (`|EnumEquality` (`self.CurrentLanePosition`) "NewEnumerator1") (not (`self.LastMovementHitNote`)))
        (`GameplayStatics.PlaySound2D` "/Game/Assets/Audio/SFX/A_SwitchLane.A_SwitchLane" 1.0 1.0 0.0 null null)))
    (:`then_3`
      (set `self.CurrentLanePosition` "NewEnumerator1")
      (set `self.IsInTransitionAnimation` true))))

(event `GoToLowerLane`
  (bind (_returnvalue_x _returnvalue_y _returnvalue_z) (`KismetMathLibrary.BreakVector` (`self.K2_GetActorLocation`)))
  (bind _upperlanez (`self.UpperLaneZ`))
  ;[0.875 1 0] Lower Lane Change
  (`|ExecutionSequence`
    (:`then_0`
      (`TimelineComponent.SetPlayRate` (`self.FastFallRoutine`) (/ 1.0 (`self.LaneChangeTime`)))
      (`|ExecutionSequence`
        (:`then_0`
          (`self.StopAutoFall`))
        (:`then_1`
          (bind (_direction _alpha) (`Timeline|FastFallRoutine` :`NewTime` (/ (- _returnvalue_z _upperlanez) (- (`self.LowerLaneZ`) _upperlanez)) :!via `SetNewTime` :!label _label_3)
            (:`Update`
              (`self.K2_SetActorLocation` (`KismetMathLibrary.MakeVector` _returnvalue_x _returnvalue_y (`KismetMathLibrary.Lerp` (`self.UpperLaneZ`) (`self.LowerLaneZ`) _alpha))))
            (:`Finished`
              (set `self.IsInTransitionAnimation` false))))
        (:`then_2`
          (goto _label_3))))
    (:`then_1`
      (`self.Invincibility` 0.3))
    (:`then_2`
      (if (and (`|EnumEquality` (`self.CurrentLanePosition`) "NewEnumerator1") (not (`self.LastMovementHitNote`)))
        (`GameplayStatics.PlaySound2D` "/Game/Assets/Audio/SFX/A_SwitchLane.A_SwitchLane" 1.0 1.0 0.0 null null)))
    (:`then_3`
      (set `self.CurrentLanePosition` "NewEnumerator0")
      (set `self.IsInTransitionAnimation` true))))

(event `AttackAnim`
  ;[1 0 0.6562] Change animation to attack
  (`PaperZDAnimInstance.JumpToNode` (`PaperZDAnimationComponent.AnimInstance` (`self.AnimationComponent`)) "Attack" "Animation Logic"))

(event `GravityFalls`
  (bind (_returnvalue_x _returnvalue_y) (`KismetMathLibrary.BreakVector` (`self.K2_GetActorLocation`)))
  ;[0.2422 1 0] Gravity auto fall, made manually to control it however I want
  (`TimelineComponent.SetPlayRate` (`self.FallRoutine`) (/ 1.0 (`self.FallTime`)))
  (bind (_direction _fallcurve) (`Timeline|FallRoutine` :!via `PlayFromStart` :!label _label_4)
    (:`Update`
      (`self.K2_SetActorLocation` (`KismetMathLibrary.MakeVector` _returnvalue_x _returnvalue_y (`KismetMathLibrary.Lerp` (`self.UpperLaneZ`) (`self.LowerLaneZ`) _fallcurve))))
    (:`Finished`
      (set `self.CurrentLanePosition` "NewEnumerator0"))))

(event `TryChangeLane`
  (params (TargetLane :type "/Game/AudioMapping/Enums/ENoteLane Enum" :default "NewEnumerator0") (ForceChange :type Boolean))
  ;[0 0.625 1] Called on lane input change received by the note receivers
  (set `self.LastMovementHitNote` ForceChange)
  (if (== (`self.NoteHeldCount`) 0)
    (if (`self.IsInTransitionAnimation`)
      (if ForceChange
        (switch `/Game/AudioMapping/Enums/ENoteLane` TargetLane :!label _label_5
          (:`NewEnumerator0`
            (`self.GoToLowerLane`))
          (:`NewEnumerator1`
            (`self.GoToUpperLane`)))
        (`self.AttackAnim`)
        (else
          (`self.SetInputBuffer` TargetLane 0.2)))
      (else
        (goto _label_5)))))

(event `StopAutoFall`
  ;[0.2422 1 0] Gravity auto fall, made manually to control it however I want
  (goto _label_4 :!via `Stop`))

(event `Hurt`
  (params (`Hurt Amount` :type Integer))
  ;[0.9219 1 0] Called when overlapping with notes (except long ones)
  (`|ExecutionSequence`
    (:`then_0`
      (message `/Game/Systems/BPI_Gamestate.AddLife` (`GameplayStatics.GetGameState`) (* `Hurt Amount` -1)))
    (:`then_1`
      (`self.Invincibility` 2.0))))

(event `SetInputBuffer`
  (params (Input :type "/Game/AudioMapping/Enums/ENoteLane Enum" :default "NewEnumerator0") (PersistenceTime :type "Float (double-precision)"))
  ;[0.8516 1 0] Simple Input Buffer for commands responsivity
  (set `self.InputBuffer` Input)
  (bind _output_get (set `self.PersistenceTimer` PersistenceTime))
  (if (> _output_get 0.0)
    (goto _label_6 :!via `Open`)
    (else
      (goto _label_6 :!via `Close`))))

(event `ReadInputBuffer`
  ;[0.8516 1 0] Simple Input Buffer for commands responsivity
  (`/Engine/EditorBlueprintResources/StandardMacros.Gate` true :!label _label_6
    (:`Exit`
      (bind _output_get (set `self.PersistenceTimer` (- (`self.PersistenceTimer`) (`GameplayStatics.GetWorldDeltaSeconds`))))
      (if (<= _output_get 0.0)
        (goto _label_6 :!via `Close`)
        (elif (not (`self.IsInTransitionAnimation`))
          (`self.TryChangeLane` (`self.InputBuffer`))
          (`self.SetInputBuffer` "NewEnumerator2"))))))

(event `self.ReceiveTick`
  (params (DeltaSeconds :type "Float (single-precision)"))
  (`self.ReadInputBuffer`))

(fn `TryReenableFall`
  (if (and (<= (`self.NoteHeldCount`) 0) (`|EnumEquality` (`self.CurrentLanePosition`) "NewEnumerator1"))
    (`self.GravityFalls`)))

(fn `UserConstructionScript`)