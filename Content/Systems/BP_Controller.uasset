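; Player controller that sets up Enhanced Input and handles quick restart and rush actions.
; On BeginPlay it adds the IMC_InputMap mapping context to the local player subsystem.
; Quick restart reopens the game level.
; Rush, marked as for future use, launches Fever through BP_GameState once the Fever meter is full.
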(event `self.ReceiveBeginPlay`
  (`EnhancedInputSubsystemInterface.AddMappingContext` (subsystem `EnhancedInputLocalPlayerSubsystem`) "/Game/Input/IMC_InputMap.IMC_InputMap" 0 (struct)))

(event `EnhancedInput|/Game/Input/IA_QuickRestart`
  (params (ActionValue :type Boolean) (ElapsedSeconds :type "Float (double-precision)") (TriggeredSeconds :type "Float (double-precision)") (InputAction :type "InputAction Object Reference" :default "/Game/Input/IA_QuickRestart.IA_QuickRestart"))
  ;[0.3125 1 0] Quick Restart
  (:`Started`
    (`GameplayStatics.OpenLevelBySoftObjectPtr` "/Game/Scenes/GameLevel.GameLevel")))

(event `EnhancedInput|/Game/Input/IA_Rush`
  (params (ActionValue :type Boolean) (ElapsedSeconds :type "Float (double-precision)") (TriggeredSeconds :type "Float (double-precision)") (InputAction :type "InputAction Object Reference" :default "/Game/Input/IA_Rush.IA_Rush"))
  (bind _asbp_game_state (cast `/Game/Systems/BP_GameState` (`GameplayStatics.GetGameState`) :!pure true))
  ;[1 0.375 0] for the future
  (:`Started`
    (if (>= (`/Game/Systems/BP_GameState.Fever` _asbp_game_state) 100)
      (`/Game/Systems/BP_GameState.LaunchFever` _asbp_game_state))))

(fn `UserConstructionScript`)