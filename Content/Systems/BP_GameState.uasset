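; Game state for a rhythm game, tracking score, combo, life, fever and per-judgment note counts.
; AddScore counts each Perfect, Good or Miss, resets combo on a miss, and scales points by precision plus combo and fever-mode bonuses.
; Life and fever are clamped, and empty life fires OnPlayerDeath.
; Combo increases through a separate call that records the maximum, and accuracy weights Good hits at half.
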(event `self.ReceiveBeginPlay`
  (set `self.Life` (`self.MaxLife`)))

(fn `AddFever`
  (params (ToAdd :type Integer))
  (returns (NewFever :type Integer))
  (bind _output_get (set `self.Fever` (`KismetMathLibrary.Clamp` (+ ToAdd (`self.Fever`)) 0 100)))
  (return _output_get))

(fn `AddLife`
  (params (LifeAmount :type Integer))
  (returns (NewLife :type Integer))
  (bind _output_get (set `self.Life` (`KismetMathLibrary.Clamp` (+ LifeAmount (`self.Life`)) 0 (`self.MaxLife`))))
  (if (<= _output_get 0)
    (`self.OnPlayerDeath`))
  (return _output_get))

(fn `AddScore`
  (params (`Base Amount` :type Integer) (Precision :type "/Game/AudioMapping/Enums/ENotePrecision Enum" :default "NewEnumerator0"))
  (returns (NewScore :type Integer))
  (locals (PrecisionMultiplier :type "Float (double-precision)") (FeverMultiplier :type "Float (double-precision)") (ComboMultiplier :type "Float (double-precision)"))
  (`|ExecutionSequence`
    (:`then_0`
      (switch `/Game/AudioMapping/Enums/ENotePrecision` Precision
        (:`NewEnumerator0`
          (set `local.PrecisionMultiplier` 1.0)
          (`/Engine/EditorBlueprintResources/StandardMacros.IncrementInt` (`self.PerfectCount`)))
        (:`NewEnumerator2`
          (set `local.PrecisionMultiplier` 0.5)
          (`/Engine/EditorBlueprintResources/StandardMacros.IncrementInt` (`self.GoodCount`)))
        (:`NewEnumerator1`
          (set `self.Combo` 0)
          (`/Engine/EditorBlueprintResources/StandardMacros.IncrementInt` (`self.MissCount`)
            (:`  `
              (return (`self.Score`)))))))
    (:`then_1`
      (if (`self.IsInFeverMode`)
        (set `local.FeverMultiplier` 1.0)
        (else
          (set `local.FeverMultiplier` 0.0))))
    (:`then_2`
      (set `local.ComboMultiplier` (+ 1 (/ (`KismetMathLibrary.Conv_IntToDouble` (`self.Combo`)) 100.0))))
    (:`then_3`
      (set `self.Score` (+ (`self.Score`) (* (* `Base Amount` (`local.PrecisionMultiplier`)) (+ (`local.ComboMultiplier`) (`local.FeverMultiplier`))))))
    (:`then_4`
      (return (`self.Score`)))))

(fn `GetAccuracy`
  (returns (Accuracy :type "Float (double-precision)"))
  (return (/ (+ (`self.PerfectCount`) (/ (`self.GoodCount`) 2.0)) (+ (`self.PerfectCount`) (`self.GoodCount`) (`self.MissCount`)))))

(fn `GetCombo`
  (returns (Combo :type Integer))
  (return (`self.Combo`)))

(fn `GetFever`
  (returns (Fever :type Integer))
  (return (`self.Fever`)))

(fn `GetLife`
  (returns (Life :type Integer))
  (return (`self.Life`)))

(fn `GetMaxCombo`
  (returns (MaxCombo :type Integer))
  (return (`self.MaxCombo`)))

(fn `GetNoteCount`
  (params (Type :type "/Game/AudioMapping/Enums/ENotePrecision Enum" :default "NewEnumerator0"))
  (returns (Count :type Integer))
  (switch `/Game/AudioMapping/Enums/ENotePrecision` Type
    (:`NewEnumerator0`
      (return (`self.PerfectCount`)))
    (:`NewEnumerator2`
      (return (`self.GoodCount`)))
    (:`NewEnumerator1`
      (return (`self.MissCount`)))))

(fn `GetPlayer`
  (returns (Player :type "/Game/Player/BP_Player Object Reference"))
  (return (`self.Player`)))

(fn `GetScore`
  (returns (Score :type Integer))
  (return (`self.Score`)))

(fn `IncreaseCombo`
  (params (ComboAmount :type Integer))
  (returns (NewCombo :type Integer))
  (bind _output_get (set `self.Combo` (+ ComboAmount (`self.Combo`))))
  (if (> _output_get (`self.MaxCombo`))
    (set `self.MaxCombo` _output_get))
  (return _output_get))

(fn `UserConstructionScript`)